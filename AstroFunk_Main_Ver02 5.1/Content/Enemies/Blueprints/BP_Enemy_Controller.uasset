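; AI controller for enemies that runs the BT_Enemy behavior tree on possession and feeds it player sightings from AI Perception.
; Perception updates go to HandleSightSense, which ignores anything other than sight stimuli from player character 0.
; It sets the TargetActor blackboard key while the player is seen, and on losing sight clears it and stores the stimulus location as LastKnownLocation.
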(event `self.ReceivePossess`
  (params (PossessedPawn :type "Pawn Object Reference"))
  (`self.RunBehaviorTree` "/Game/Enemies/Blueprints/BT_Enemy.BT_Enemy"))

(event `self.AIPerception.OnTargetPerceptionUpdated`
  (params (Actor :type "Actor Object Reference") (Stimulus :type "AIStimulus Structure"))
  (`self.HandleSightSense` Actor Stimulus))

(fn `HandleSightSense`
  (params (Actor :type "Actor Object Reference") (Stimulus :type "AIStimulus Structure"))
  (bind (_stimulus_age _stimulus_expirationage _stimulus_strength _stimulus_stimuluslocation _stimulus_receiverlocation _stimulus_tag _stimulus_bsuccessfullysensed) (break `AIStimulus` (`local.Stimulus`)))
  (bind _returnvalue (`AIPerceptionSystem.GetSenseClassForStimulus` Stimulus))
  (if (== _returnvalue "/Script/AIModule.AISense_Sight")
    (if (== (`local.Actor`) (`GameplayStatics.GetPlayerCharacter` 0))
      (`BlackboardComponent.SetValueAsObject` (`self.Blackboard_Enemy`) "TargetActor" (`KismetMathLibrary.SelectObject` (`GameplayStatics.GetPlayerCharacter` 0) null _stimulus_bsuccessfullysensed))
      (if (not _stimulus_bsuccessfullysensed)
        (`BlackboardComponent.SetValueAsVector` (`self.Blackboard_Enemy`) "LastKnownLocation" _stimulus_stimuluslocation))
      (else
        (return)))
    (else
      (return))))

(fn `UserConstructionScript`)